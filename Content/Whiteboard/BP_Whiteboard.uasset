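; Whiteboard actor that takes marker input, paints it onto a render target and shows a number for each finished drawing.
; BeginPlay clears RT_Whiteboard and creates a dynamic marker material, which each draw call stamps at the given 2D location.
; Stroke events also feed a child DrawingBoard actor that records, ends or discards contours.
; FinishDrawing increments a shape count and sends the board's FinishContour result to a NumberDisplay widget.
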(event `self.ReceiveBeginPlay`
  (bind _returnvalue (`KismetMaterialLibrary.CreateDynamicMaterialInstance` "/Game/Whiteboard/M_Marker.M_Marker"))
  (set `self.WhieteboardMarker_Mi` _returnvalue)
  (`KismetRenderingLibrary.ClearRenderTarget2D` "/Game/Whiteboard/RT_Whiteboard.RT_Whiteboard"))

(event `Draw On Whiteboard`
  (params (`Location To Draw` :type "Vector2D Structure"))
  (bind _whieteboardmarker_mi (`self.WhieteboardMarker_Mi`))
  (bind _asdrawing_board (cast `DrawingBoard` (`ChildActorComponent.ChildActor` (`self.DrawingBoard`))))
  (`DrawingBoard.AddDot` _asdrawing_board `Location To Draw`)
  (`MaterialInstanceDynamic.SetVectorParameterValue` _whieteboardmarker_mi "DrawLocation" (`KismetMathLibrary.Conv_VectorToLinearColor` (`KismetMathLibrary.Conv_Vector2DToVector` `Location To Draw`)))
  (`KismetRenderingLibrary.DrawMaterialToRenderTarget` "/Game/Whiteboard/RT_Whiteboard.RT_Whiteboard" _whieteboardmarker_mi))

(event `Begin Drawing`
  (bind _asdrawing_board (cast `DrawingBoard` (`ChildActorComponent.ChildActor` (`self.DrawingBoard`))))
  (`DrawingBoard.BeginContour` _asdrawing_board))

(event `End Stroke`
  (bind _asdrawing_board (cast `DrawingBoard` (`ChildActorComponent.ChildActor` (`self.DrawingBoard`))))
  (`DrawingBoard.EndStroke` _asdrawing_board))

(event `Discard`
  (bind _asdrawing_board (cast `DrawingBoard` (`ChildActorComponent.ChildActor` (`self.DrawingBoard`))))
  (`DrawingBoard.DiscardContour` _asdrawing_board)
  (`KismetSystemLibrary.PrintString` "Succesfully discarded!"))

(event `Finish Drawing`
  (bind _asdrawing_board (cast `DrawingBoard` (`ChildActorComponent.ChildActor` (`self.DrawingBoard`))))
  (bind _returnvalue (`DrawingBoard.FinishContour` _asdrawing_board))
  (bind _asnumber_display (cast `/Game/Whiteboard/NumberDisplay` (`WidgetComponent.GetUserWidgetObject` (`self.Widget`))))
  (`/Engine/EditorBlueprintResources/StandardMacros.IncrementInt` (`self.ShapesDrawn`)
    (:`  `
      (`/Game/Whiteboard/NumberDisplay.SetNumber` _asnumber_display _returnvalue))))

(fn `UserConstructionScript`)